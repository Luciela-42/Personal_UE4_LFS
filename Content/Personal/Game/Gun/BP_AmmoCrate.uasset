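; BP_AmmoCrate is an ammo pickup that the player collects by pressing Interact nearby.
; Overlap of its Box by Ue4ASP_Character toggles the crate's input and a Gate, so Interact only works inside.
; Interacting adds a randomly selected amount to player 0's Ammo, then destroys the crate.
; The random range covers three of the four Select options, so the largest amount never drops.
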(event `InputAction|Interact`
  (params (Key :type "Key Structure"))
  (:`Pressed`
    (`/Engine/EditorBlueprintResources/StandardMacros.Gate` true :!label _label
      (:`Exit`
        (bind _asue_4asp_character (cast `/Game/Personal/Anim/Ue4ASP_Character` (`GameplayStatics.GetPlayerCharacter` 0)))
        (set `/Game/Personal/Anim/Ue4ASP_Character.Ammo` (+ (`/Game/Personal/Anim/Ue4ASP_Character.Ammo` _asue_4asp_character) (select `int` (`KismetMathLibrary.RandomInteger` 3) :`0` 15 :`1` 20 :`2` 25 :`3` 30)) _asue_4asp_character)
        (`self.K2_DestroyActor`)))))

(event `self.Box.OnComponentBeginOverlap`
  (params (OverlappedComponent :type "PrimitiveComponent Object Reference") (OtherActor :type "Actor Object Reference") (OtherComp :type "PrimitiveComponent Object Reference") (OtherBodyIndex :type Integer) (bFromSweep :type Boolean) (SweepResult :type "HitResult Structure (by ref)"))
  (cast `/Game/Personal/Anim/Ue4ASP_Character` OtherActor)
  (`self.EnableInput` (`GameplayStatics.GetPlayerController` 0))
  (goto _label :!via `Open`))

(event `self.Box.OnComponentEndOverlap`
  (params (OverlappedComponent :type "PrimitiveComponent Object Reference") (OtherActor :type "Actor Object Reference") (OtherComp :type "PrimitiveComponent Object Reference") (OtherBodyIndex :type Integer))
  (cast `/Game/Personal/Anim/Ue4ASP_Character` OtherActor)
  (`self.DisableInput` (`GameplayStatics.GetPlayerController` 0))
  (goto _label :!via `Close`))

(fn `UserConstructionScript`)
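; BP_HealthPack is an interactable health pickup that restores a fixed amount of the player character's health, clamped to MaxHealth.
; Box overlap by a Ue4ASP_Character enables input, shows a prompt widget and opens a Gate, and leaving reverses all three.
; Pressing Interact while the gate is open plays a 2D sound, heals player 0's character and destroys the pack.
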(event `self.ReceiveBeginPlay`
  (`SceneComponent.SetVisibility` (`self.Widget`) false false))

(event `InputAction|Interact`
  (params (Key :type "Key Structure"))
  (:`Pressed`
    (`/Engine/EditorBlueprintResources/StandardMacros.Gate` true :!label _label
      (:`Exit`
        (`GameplayStatics.PlaySound2D` "/Game/MilitaryWeapDark/Sound/Pistol/Pistol_MagEject_Cue.Pistol_MagEject_Cue" 1.0 1.0 0.0 null null)
        (bind _asue_4asp_character (cast `/Game/Personal/Anim/Ue4ASP_Character` (`GameplayStatics.GetPlayerCharacter` 0)))
        (set `/Game/Personal/Anim/Ue4ASP_Character.Health` (`KismetMathLibrary.FClamp` (+ (`/Game/Personal/Anim/Ue4ASP_Character.Health` _asue_4asp_character) 70.0) 0.0 (`/Game/Personal/Anim/Ue4ASP_Character.MaxHealth` _asue_4asp_character)) _asue_4asp_character)
        (`self.K2_DestroyActor`)))))

(event `self.Box.OnComponentBeginOverlap`
  (params (OverlappedComponent :type "PrimitiveComponent Object Reference") (OtherActor :type "Actor Object Reference") (OtherComp :type "PrimitiveComponent Object Reference") (OtherBodyIndex :type Integer) (bFromSweep :type Boolean) (SweepResult :type "HitResult Structure (by ref)"))
  (cast `/Game/Personal/Anim/Ue4ASP_Character` OtherActor)
  (`self.EnableInput` (`GameplayStatics.GetPlayerController` 0))
  (`SceneComponent.SetVisibility` (`self.Widget`) true false)
  (goto _label :!via `Open`))

(event `self.Box.OnComponentEndOverlap`
  (params (OverlappedComponent :type "PrimitiveComponent Object Reference") (OtherActor :type "Actor Object Reference") (OtherComp :type "PrimitiveComponent Object Reference") (OtherBodyIndex :type Integer))
  (cast `/Game/Personal/Anim/Ue4ASP_Character` OtherActor)
  (`self.DisableInput` (`GameplayStatics.GetPlayerController` 0))
  (`SceneComponent.SetVisibility` (`self.Widget`) false false)
  (goto _label :!via `Close`))

(fn `UserConstructionScript`)
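; Sliding double glass door that the player toggles with the Interact input while holding a key.
; Trigger overlap by the player character enables input and opens a Gate; leaving disables both.
; With HasKey, it plays an access sound and, after a short delay, a FlipFlop plays or reverses a Timeline lerping both panels.
; Without the key, it briefly shows a widget.
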(event `self.ReceiveBeginPlay`
  (`SceneComponent.SetVisibility` (`self.Widget`) false false))

(event `InputAction|Interact`
  (params (Key :type "Key Structure"))
  (bind _widget (`self.Widget`))
  (:`Pressed`
    (if (`/Game/Personal/Anim/Ue4ASP_Character.HasKey?` (stale `self.Trigger.OnComponentBeginOverlap` _asue_4asp_character))
      (`GameplayStatics.PlaySound2D` "/Game/Personal/Game/Level/interactActor/Access_Cue.Access_Cue" 1.0 1.0 0.0 null null)
      (`KismetSystemLibrary.Delay` 0.5)
      (`/Engine/EditorBlueprintResources/StandardMacros.Gate` true :!label _label
        (:`Exit`
          (`/Engine/EditorBlueprintResources/StandardMacros.FlipFlop`
            (:`A`
              (bind (_direction `_새_트랙_0`) (`Timeline|DoorOpen` :!label _label_2)
                (:`Update`
                  (`|ExecutionSequence`
                    (:`then_0`
                      (`SceneComponent.K2_SetRelativeLocation` (`self.SM_GlassDoor_A`) (`KismetMathLibrary.VLerp` (`self.Door Closed A`) (`self.Door Open A`) `_새_트랙_0`) false false))
                    (:`then_1`
                      (`SceneComponent.K2_SetRelativeLocation` (`self.SM_GlassDoor_B`) (`KismetMathLibrary.VLerp` (`self.Door Closed B`) (`self.Door Open B`) `_새_트랙_0`) false false))))))
            (:`B`
              (goto _label_2 :!via `Reverse`)))))
      (else
        (`SceneComponent.SetVisibility` _widget true false)
        (`KismetSystemLibrary.Delay` 1.0)
        (`SceneComponent.SetVisibility` _widget false false)))))

(event `self.Trigger.OnComponentBeginOverlap`
  (params (OverlappedComponent :type "PrimitiveComponent Object Reference") (OtherActor :type "Actor Object Reference") (OtherComp :type "PrimitiveComponent Object Reference") (OtherBodyIndex :type Integer) (bFromSweep :type Boolean) (SweepResult :type "HitResult Structure (by ref)"))
  (bind _asue_4asp_character (cast `/Game/Personal/Anim/Ue4ASP_Character` OtherActor))
  (`self.EnableInput` (`GameplayStatics.GetPlayerController` 0))
  (goto _label :!via `Open`))

(event `self.Trigger.OnComponentEndOverlap`
  (params (OverlappedComponent :type "PrimitiveComponent Object Reference") (OtherActor :type "Actor Object Reference") (OtherComp :type "PrimitiveComponent Object Reference") (OtherBodyIndex :type Integer))
  (cast `/Game/Personal/Anim/Ue4ASP_Character` OtherActor)
  (`self.DisableInput` (`GameplayStatics.GetPlayerController` 0))
  (goto _label :!via `Close`))

(fn `UserConstructionScript`)
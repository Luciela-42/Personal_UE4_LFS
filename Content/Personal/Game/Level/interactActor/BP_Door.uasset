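; BP_Door is an automatic double glass sliding door that opens when something enters its trigger.
; Begin overlap on the Trigger plays the DoorOpen timeline, and end overlap reverses it to close.
; Each timeline update lerps both door meshes between their closed and open relative locations, without sweep.
; Overlaps are not filtered by actor, and any single exit starts closing the door.
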(event `self.Trigger.OnComponentBeginOverlap`
  (params (OverlappedComponent :type "PrimitiveComponent Object Reference") (OtherActor :type "Actor Object Reference") (OtherComp :type "PrimitiveComponent Object Reference") (OtherBodyIndex :type Integer) (bFromSweep :type Boolean) (SweepResult :type "HitResult Structure (by ref)"))
  (bind (_direction `_새_트랙_0`) (`Timeline|DoorOpen` :!label _label)
    (:`Update`
      (`|ExecutionSequence`
        (:`then_0`
          (`SceneComponent.K2_SetRelativeLocation` (`self.SM_GlassDoor_A`) (`KismetMathLibrary.VLerp` (`self.Door Closed A`) (`self.Door Open A`) `_새_트랙_0`) false false))
        (:`then_1`
          (`SceneComponent.K2_SetRelativeLocation` (`self.SM_GlassDoor_B`) (`KismetMathLibrary.VLerp` (`self.Door Closed B`) (`self.Door Open B`) `_새_트랙_0`) false false))))))

(event `self.Trigger.OnComponentEndOverlap`
  (params (OverlappedComponent :type "PrimitiveComponent Object Reference") (OtherActor :type "Actor Object Reference") (OtherComp :type "PrimitiveComponent Object Reference") (OtherBodyIndex :type Integer))
  (goto _label :!via `Reverse`))

(fn `UserConstructionScript`)
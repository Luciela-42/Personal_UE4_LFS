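; BP_MainDoor is an interactable main door that a Ue4ASP_Character can open and close with the Interact input if it holds the main key.
; A trigger overlap enables input and opens a Gate, and leaving reverses both.
; With the key, a sound and short delay precede the Gate, then a FlipFlop plays or reverses a timeline lerping the mesh between closed and open positions.
; Without it, Widget1 appears briefly.
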(event `self.ReceiveBeginPlay`
  (`SceneComponent.SetVisibility` (`self.Widget1`) false false))

(event `InputAction|Interact`
  (params (Key :type "Key Structure"))
  (bind _widget1 (`self.Widget1`))
  (:`Pressed`
    (if (`/Game/Personal/Anim/Ue4ASP_Character.HasMainKey?` (stale `self.Trigger.OnComponentBeginOverlap` _asue_4asp_character))
      (`GameplayStatics.PlaySound2D` "/Game/Personal/Game/Level/interactActor/AccessMain_Cue.AccessMain_Cue" 1.0 1.0 0.0 null null)
      (`KismetSystemLibrary.Delay` 0.5)
      (`/Engine/EditorBlueprintResources/StandardMacros.Gate` true :!label _label
        (:`Exit`
          (`/Engine/EditorBlueprintResources/StandardMacros.FlipFlop`
            (:`A`
              (bind (_direction `_새_트랙_0`) (`Timeline|타임라인_0` :!label _label_2)
                (:`Update`
                  (`SceneComponent.K2_SetRelativeLocation` (`self.StaticMesh`) (`KismetMathLibrary.VLerp` (`self.Door Closed`) (`self.Door Open`) `_새_트랙_0`) false false))))
            (:`B`
              (goto _label_2 :!via `Reverse`)))))
      (else
        (`SceneComponent.SetVisibility` _widget1 true false)
        (`KismetSystemLibrary.Delay` 1.0)
        (`SceneComponent.SetVisibility` _widget1 false false)))))

(event `self.Trigger.OnComponentBeginOverlap`
  (params (OverlappedComponent :type "PrimitiveComponent Object Reference") (OtherActor :type "Actor Object Reference") (OtherComp :type "PrimitiveComponent Object Reference") (OtherBodyIndex :type Integer) (bFromSweep :type Boolean) (SweepResult :type "HitResult Structure (by ref)"))
  (bind _asue_4asp_character (cast `/Game/Personal/Anim/Ue4ASP_Character` OtherActor))
  (`self.EnableInput` (`GameplayStatics.GetPlayerController` 0))
  (goto _label :!via `Open`))

(event `self.Trigger.OnComponentEndOverlap`
  (params (OverlappedComponent :type "PrimitiveComponent Object Reference") (OtherActor :type "Actor Object Reference") (OtherComp :type "PrimitiveComponent Object Reference") (OtherBodyIndex :type Integer))
  (cast `/Game/Personal/Anim/Ue4ASP_Character` OtherActor)
  (`self.DisableInput` (`GameplayStatics.GetPlayerController` 0))
  (goto _label :!via `Close`))

(fn `UserConstructionScript`)
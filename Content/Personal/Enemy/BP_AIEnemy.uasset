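; AI enemy character that detects the player, takes damage and may drop a health pack on death.
; PawnSensing and hits set EnemyFound, a forward line trace sets ActiveDetect, and CheckPlayerDead clears the found and hit flags.
; Interface damage makes headshots lethal; death plays a random animation, disables collision and destroys the actor after a delay.
; Drops use weighted chance and a downward trace for placement; DropAmmo is defined but never called here.
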(event `self.ReceiveBeginPlay`
  (set `self.CurrentHealth` (`self.MaxHealth`)))

(event `/Game/Personal/Enemy/TakeDamage.I_TakeDamage`
  (params (Bone :type Name) (Damage :type "Float (single-precision)"))
  (if (== Bone "head")
    (`GameplayStatics.PlaySound2D` "/Game/MilitaryWeapDark/Sound/Rifle/Rifle_ImpactBody_Cue.Rifle_ImpactBody_Cue" 1.0 1.0 0.0 null null)
    (`KismetSystemLibrary.PrintString` "Head Shot")
    (set `self.CurrentHealth` 0.0)
    (else
      (set `self.EnemyFound` true)
      (set `self.EnemyHit?` true)
      (bind _output_get (set `self.CurrentHealth` (- (`self.CurrentHealth`) Damage)))))
  (if (<= _output_get 0.0)
    (set `self.IsDeath?` true)
    (`GameplayStatics.PlaySoundAtLocation` "/Game/Personal/Enemy/DeadCue.DeadCue" (`self.K2_GetActorLocation`) (struct) 1.0 1.0 0.0 null null null)
    (`CharacterMovementComponent.DisableMovement` (`self.CharacterMovement`))
    (`SkeletalMeshComponent.PlayAnimation` (`self.Mesh`) (select `int` (`KismetMathLibrary.RandomInteger` 6) :`0` "/Game/Personal/Anim/HitAndDead/Death_1_Montage.Death_1_Montage" :`1` "/Game/Personal/Anim/HitAndDead/Death_2_Montage.Death_2_Montage" :`2` "/Game/Personal/Anim/HitAndDead/Death_3_Montage.Death_3_Montage" :`3` "/Game/Personal/Anim/HitAndDead/Death_4_Montage.Death_4_Montage" :`4` "/Game/Personal/Anim/HitAndDead/Dead_1_Montage.Dead_1_Montage" :`5` "/Game/Personal/Anim/HitAndDead/Dead_2_Montage.Dead_2_Montage" :`6` "/Game/Personal/Anim/HitAndDead/Dead_3_Montage.Dead_3_Montage" :!type "AnimMontage Object Reference") false)
    (`self.SetActorEnableCollision` false)
    (`|ExecutionSequence`
      (:`then_0`
        (`self.DropHealthPack`))
      (:`then_1`
        (`KismetSystemLibrary.Delay` 5.0)
        (`self.K2_DestroyActor`)))
    (else
      (`GameplayStatics.PlaySound2D` "/Game/Personal/Enemy/Hit.Hit" 1.0 1.0 0.0 null null))))

(event `CheckPlayerDead`
  (bind _asue_4asp_character (cast `/Game/Personal/Anim/Ue4ASP_Character` (`GameplayStatics.GetPlayerCharacter` 0)))
  (if (`/Game/Personal/Anim/Ue4ASP_Character.IsDead?` _asue_4asp_character)
    (set `self.EnemyHit?` false)
    (set `self.EnemyFound` false)))

(event `self.PawnSensing.OnSeePawn`
  (params (Pawn :type "Pawn Object Reference"))
  (bind _asue_4asp_character (cast `/Game/Personal/Anim/Ue4ASP_Character` Pawn))
  (if (not (`/Game/Personal/Anim/Ue4ASP_Character.IsDead?` _asue_4asp_character))
    (set `self.EnemyFound` true)))

(event `ScanEnemy`
  (bind _visiondirection (`self.VisionDirection`))
  (bind _returnvalue (`SceneComponent.K2_GetComponentLocation` _visiondirection))
  (bind (_outhit _returnvalue_2) (`KismetSystemLibrary.LineTraceSingle` _returnvalue (+ _returnvalue (* (`SceneComponent.GetForwardVector` _visiondirection) 3000.0)) "TraceTypeQuery1" true (`|MakeArray` self :!type "Actor Object Reference")))
  (if _returnvalue_2
    (bind (_bblockinghit _binitialoverlap _time _distance _location _impactpoint _normal _impactnormal _physmat _hitactor) (`GameplayStatics.BreakHitResult` _outhit))
    (if (`KismetSystemLibrary.DoesImplementInterface` _hitactor "/Game/Personal/Enemy/TakeDamage.TakeDamage_C")
      (cast `/Game/Personal/Anim/Ue4ASP_Character` _hitactor)
      (set `self.ActiveDetect` true)
      (else
        (set `self.ActiveDetect` false)))))

(fn `DropAmmo`
  (bind _returnvalue (`self.K2_GetActorLocation`))
  (if (`KismetMathLibrary.RandomBoolWithWeight` 0.55)
    (bind _outhit (`KismetSystemLibrary.LineTraceSingle` _returnvalue (- _returnvalue (0.0 0.0 1500.0)) "TraceTypeQuery1"))
    (`|SpawnActorFromClass` "/Game/Personal/Game/Gun/BP_AmmoCrate.BP_AmmoCrate_C" (`KismetMathLibrary.MakeTransform` (`.Location` (`GameplayStatics.BreakHitResult` _outhit))) "Undefined" "OverrideRootScale" null null)))

(fn `DropHealthPack`
  (bind _returnvalue (`self.K2_GetActorLocation`))
  (if (`KismetMathLibrary.RandomBoolWithWeight` 0.8)
    (bind _outhit (`KismetSystemLibrary.LineTraceSingle` _returnvalue (- _returnvalue (0.0 0.0 1500.0)) "TraceTypeQuery1"))
    (`|SpawnActorFromClass` "/Game/Personal/Game/Player/BP_HealthPack.BP_HealthPack_C" (`KismetMathLibrary.MakeTransform` (+ (`.Location` (`GameplayStatics.BreakHitResult` _outhit)) (50.0 0.0 0.0))) "Undefined" "OverrideRootScale" null null)))

(fn `UserConstructionScript`)
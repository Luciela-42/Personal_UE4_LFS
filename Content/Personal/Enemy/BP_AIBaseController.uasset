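; AI controller for BP_AIEnemy that patrols waypoints and switches to hunting the player once the pawn reports an enemy found.
; Patrol moves back and forth along the pawn's waypoint array with a pause at each stop.
; A looping timer polls the detection flag to trigger the chase and stops when the pawn dies.
; Reaching the player fires a debug-drawn muzzle line trace, whose hit result is not yet used.
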(event `self.ReceiveBeginPlay`
  (bind _asbp_aienemy (cast `/Game/Personal/Enemy/BP_AIEnemy` (`self.K2_GetPawn`)))
  (set `self.AIBaseREF` _asbp_aienemy)
  (set `self.Waypoints` (`/Game/Personal/Enemy/BP_AIEnemy.Waypoints` _asbp_aienemy))
  (bind _returnvalue (`KismetSystemLibrary.K2_SetTimer` null "CheckState" 0.3 true))
  (set `self.ClearTimer` _returnvalue)
  (`|AIMoveTo` _asbp_aienemy (0.0 0.0 0.0) (`|GetArrayItem` (`self.Waypoints`) (`self.CurrentWaypoint`))
    (:`OnSuccess`
      (`KismetSystemLibrary.Delay` 4.0)
      (`self.Patrolling`))))

(event `Patrolling`
  (if (not (`self.FoundEnemy`))
    (if (`self.WalkBack`)
      (`/Engine/EditorBlueprintResources/StandardMacros.DecrementInt` (`self.CurrentWaypoint`)
        (:`  `
          (`|AIMoveTo` null (0.0 0.0 0.0) (`|GetArrayItem` (`self.Waypoints`) (`self.CurrentWaypoint`))
            (:`OnSuccess`
              (if (<= (`self.CurrentWaypoint`) 0)
                (set `self.WalkBack` false))))))
      (else
        (`/Engine/EditorBlueprintResources/StandardMacros.IncrementInt` (`self.CurrentWaypoint`)
          (:`  `
            (`|AIMoveTo` null (0.0 0.0 0.0) (`|GetArrayItem` (`self.Waypoints`) (`self.CurrentWaypoint`))
              (:`OnSuccess`
                (if (>= (`self.CurrentWaypoint`) (- (`KismetArrayLibrary.Array_Length` (`self.Waypoints`)) 1))
                  (set `self.WalkBack` true))))))))
    (`KismetSystemLibrary.Delay` 4.0)
    (`self.Patrolling`)))

(event `CheckState`
  (bind _aibaseref (`self.AIBaseREF`))
  (if (`/Game/Personal/Enemy/BP_AIEnemy.IsDeath?` _aibaseref)
    (`KismetSystemLibrary.K2_ClearAndInvalidateTimerHandle` (`self.ClearTimer`))
    (else
      (bind _output_get (set `self.FoundEnemy` (`/Game/Personal/Enemy/BP_AIEnemy.EnemyFound` _aibaseref)))
      (if _output_get
        (`self.OnHunt`)))))

(event `OnHunt`
  (`|AIMoveTo` null (0.0 0.0 0.0) (`GameplayStatics.GetPlayerCharacter` 0) 1000.0 true
    (:`OnSuccess`
      (`self.Fire`))))

(event `Fire`
  (bind _sk_ka47 (`/Game/Personal/Enemy/BP_AIEnemy.SK_KA47` (`self.AIBaseREF`)))
  (bind _returnvalue (`SceneComponent.GetSocketLocation` _sk_ka47 "Muzzle"))
  (bind (_outhit _returnvalue_2) (`KismetSystemLibrary.LineTraceSingle` :`Start` _returnvalue :`End` (+ _returnvalue (* (`SceneComponent.GetRightVector` _sk_ka47) 15000.0)) :`TraceChannel` "TraceTypeQuery2" :`bTraceComplex` true :`DrawDebugType` "ForDuration"))
  (if _returnvalue_2
    _))

(fn `UserConstructionScript`)
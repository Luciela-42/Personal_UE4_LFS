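; Enemy Blueprint with health, hit reactions, death and ammo drops.
; Damage triggers sound and a random montage, briefly halting movement; at zero health it disables collision, maybe drops BP_AmmoCrate at a downward trace hit, and destroys itself after a delay.
; ChasePlayer loops AIMoveTo on the player until death, but its initial call and random walk-speed setup are unconnected, so the chase never starts here.
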(event `self.ReceiveBeginPlay`)

(event `ChasePlayer`
  (params (`Chase Player` :type "/Game/Personal/Anim/Ue4ASP_Character Object Reference"))
  (if (not (`self.IsDead?`))
    (`|AIMoveTo` self (0.0 0.0 0.0) `Chase Player`
      (:`OnSuccess`
        _)
      (:`OnFail`
        _))
    (`self.ChasePlayer` (`self.Char REF`))))

(event `self.ReceiveAnyDamage`
  (params (Damage :type "Float (single-precision)") (DamageType :type "DamageType Object Reference") (InstigatedBy :type "Controller Object Reference") (DamageCauser :type "Actor Object Reference"))
  (bind _returnvalue (`self.K2_GetActorLocation`))
  (if (not (`self.IsDead?`))
    (bind _output_get (set `self.Health` (`KismetMathLibrary.FClamp` (- (`self.Health`) Damage) 0.0 100.0))) ; Health의 기본 값을 100으로 설정하여 받은 데미지를 빼 Health에 다시 반환한다
    (if (== _output_get 0.0)
      (`GameplayStatics.PlaySoundAtLocation` "/Game/Personal/Enemy/DeadCue.DeadCue" _returnvalue (struct) 1.0 1.0 0.0 null null null)
      (`CharacterMovementComponent.DisableMovement` (`self.CharacterMovement`))
      (set `self.IsDead?` true)
      (`self.PlayAnimMontage` (select `int` (`KismetMathLibrary.RandomInteger` 6) :`0` "/Game/Personal/Anim/HitAndDead/Death_1_Montage.Death_1_Montage" :`1` "/Game/Personal/Anim/HitAndDead/Death_2_Montage.Death_2_Montage" :`2` "/Game/Personal/Anim/HitAndDead/Death_3_Montage.Death_3_Montage" :`3` "/Game/Personal/Anim/HitAndDead/Death_4_Montage.Death_4_Montage" :`4` "/Game/Personal/Anim/HitAndDead/Dead_1_Montage.Dead_1_Montage" :`5` "/Game/Personal/Anim/HitAndDead/Dead_2_Montage.Dead_2_Montage" :`6` "/Game/Personal/Anim/HitAndDead/Dead_3_Montage.Dead_3_Montage" :!type "AnimMontage Object Reference"))
      (`PrimitiveComponent.SetCollisionEnabled` (`self.CapsuleComponent`) "NoCollision")
      (`PrimitiveComponent.SetCollisionEnabled` (`self.Mesh`) "NoCollision") ; 적이 죽었을때 캐릭터 메쉬와 캡슐 콜리전을 꺼 그 위를 지나다닐수 있도록 설정
      (`|ExecutionSequence`
        (:`then_0`
          (`self.DropAmmo`))
        (:`then_1`
          (`KismetSystemLibrary.Delay` 10.0)
          (`self.K2_DestroyActor`)))
      (else
        (set `self.EnemyFound` true)
        (`GameplayStatics.PlaySoundAtLocation` "/Game/Personal/Enemy/Hit.Hit" _returnvalue (struct) 1.0 1.0 0.0 null null null)
        (`CharacterMovementComponent.DisableMovement` (`self.CharacterMovement`))
        (bind _returnvalue_2 (`self.PlayAnimMontage` (select `int` (`KismetMathLibrary.RandomInteger` 3) :`0` "/Game/Personal/Anim/HitAndDead/Hit_1_Montage.Hit_1_Montage" :`1` "/Game/Personal/Anim/HitAndDead/Hit_2_Montage.Hit_2_Montage" :`2` "/Game/Personal/Anim/HitAndDead/Hit_3_Montage.Hit_3_Montage" :`3` "/Game/Personal/Anim/HitAndDead/Hit_4_Montage.Hit_4_Montage" :`4` "/Game/Personal/Anim/HitAndDead/Hit_React_1_Montage.Hit_React_1_Montage" :`5` "/Game/Personal/Anim/HitAndDead/Hit_React_2_Montage.Hit_React_2_Montage" :`6` "/Game/Personal/Anim/HitAndDead/Hit_React_3_Montage.Hit_React_3_Montage" :`7` "/Game/Personal/Anim/HitAndDead/Hit_React_4_Montage.Hit_React_4_Montage" :!type "AnimMontage Object Reference")))
        (`KismetSystemLibrary.Delay` _returnvalue_2)
        (if (not (`self.IsDead?`))
          (`CharacterMovementComponent.SetMovementMode` (`self.CharacterMovement`) "MOVE_Walking" 0))))))

(fn `DropAmmo`
  (bind _returnvalue (`self.K2_GetActorLocation`))
  (if (`KismetMathLibrary.RandomBoolWithWeight` 0.55)
    (bind _outhit (`KismetSystemLibrary.LineTraceSingle` _returnvalue (- _returnvalue (0.0 0.0 1500.0)) "TraceTypeQuery1"))
    (`|SpawnActorFromClass` "/Game/Personal/Game/Gun/BP_AmmoCrate.BP_AmmoCrate_C" (`KismetMathLibrary.MakeTransform` (`.Location` (`GameplayStatics.BreakHitResult` _outhit))) "Undefined" "OverrideRootScale" null null)))

(fn `UserConstructionScript`)